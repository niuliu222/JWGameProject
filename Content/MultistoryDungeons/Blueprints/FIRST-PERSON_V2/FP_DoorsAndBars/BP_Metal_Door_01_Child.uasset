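; Metal door child Blueprint that adds story-event gating for the Catch_0004 dialogue sequence.
; While Catch_0004 is flagged, Tick closes an open door once via the OpenDoor timeline, or plays it open once when the saver's EventCatch02CanOpenDoor is set.
; Once Catch_0004_01 is flagged, player input reaches the parent only with that saved flag; otherwise a notification says a mechanism must be opened.
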(event `self.ReceiveTick`
  (params (DeltaSeconds :type "Float (single-precision)"))
  (`parent.ReceiveTick` DeltaSeconds)
  (bind _true_if_happen (`/Game/Envoronments/Dlg/DlgLib.QueryDialogureHappen` "Catch_0004"))
  (if _true_if_happen
    (if (`self.bOpen`)
      (if (not (`self.bReverse`))
        (`TimelineComponent.Reverse` (`self.open door`))
        (set `self.bReverse` true)
        (set `self.bOpen` false))
      (else
        (bind _gamesaver (`/Game/JW/WorldMemory/WorldMemoryLibrary.GetJWGameSaver`))
        (if (`/Game/JW/WorldMemory/GameSave/JWSaveGame.bEvent_Catch02_CanOpenDoor` _gamesaver)
          (if (not (`self.bPlayFromStart`))
            (`TimelineComponent.PlayFromStart` (`self.open door`))
            (set `self.bPlayFromStart` true)))))))

(event `self.InputOnInput`
  (bind _true_if_happen (`/Game/Envoronments/Dlg/DlgLib.QueryDialogureHappen` "Catch_0004_01"))
  (if _true_if_happen
    (bind _gamesaver (`/Game/JW/WorldMemory/WorldMemoryLibrary.GetJWGameSaver`))
    (if (`/Game/JW/WorldMemory/GameSave/JWSaveGame.bEvent_Catch02_CanOpenDoor` _gamesaver)
      (`parent.InputOnInput`)
      (else
        (bind _umg_controller (`/Game/Envoronments/UMG/UMG.GetUMGController`))
        (`/Game/Envoronments/UMG/UmgController.SetNotificationText` _umg_controller "需要打开机关" "无法打开")))
    (else
      (`parent.InputOnInput`))))

(fn `UserConstructionScript`
  (`parent.UserConstructionScript`))