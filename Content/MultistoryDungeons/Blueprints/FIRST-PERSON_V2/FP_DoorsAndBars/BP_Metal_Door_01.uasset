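; Locked double metal door that the player opens with an interact prompt, spending one key collectable.
; Input checks the CollectID count, decrements it or shows a no-key notification, then plays a timeline that rotates both leaves.
; The unlock is saved to the world saver's BoolMap under SaveName, auto-filled with a GUID in construction when empty.
; Loading restores only the unlocked flag, so reopening needs input but no key.
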(event `OnOpen`
  (`TimelineComponent.Play` (`self.open door`)))

(event `/Game/Envoronments/Types/Interface/InputableInterface.InputOnInput`
  (if (`self.bOpenedBefore`)
    (if (not (`self.bOpen`))
      (`self.OnOpen`))
    (else
      (bind _num (`/Game/JW/WorldMemory/WorldMemoryLibrary.GetCollectableObjectNumber` (`self.CollectID`)))
      (if (> _num 0)
        (`/Game/JW/WorldMemory/WorldMemoryLibrary.SetCollectableObjectNumber` (`self.CollectID`) (- _num 1))
        (bind _worldmemory (`/Game/JW/WorldMemory/WorldMemoryLibrary.GetWorldMemory`))
        (`BlueprintMapLibrary.Map_Add` (`/Game/JW/WorldMemory/GameSave/JWSaveGame.BoolMap` (`/Game/JW/WorldMemory/WorldMemory.GameSaver` _worldmemory)) (`self.SaveName`) true)
        (set `self.bOpenedBefore` true)
        (`self.OnOpen`)
        (set `self.bOpen` true)
        (bind _umg_controller (`/Game/Envoronments/UMG/UMG.GetUMGController`))
        (`/Game/Envoronments/UMG/UmgController.UnSetNotificationText` _umg_controller)
        (else
          (bind _umg_controller_2 (`/Game/Envoronments/UMG/UMG.GetUMGController`))
          (`/Game/Envoronments/UMG/UmgController.SetNotificationText` _umg_controller_2 "无法打开" "没有钥匙"))))))

(event `/Game/Envoronments/Types/Interface/Saveable.OnSaverLoad`
  (params (Saver :type "/Game/JW/WorldMemory/GameSave/JWSaveGame Object Reference"))
  (bind (_value _returnvalue) (`BlueprintMapLibrary.Map_Find` (`/Game/JW/WorldMemory/GameSave/JWSaveGame.BoolMap` Saver) (`self.SaveName`)))
  (set `self.bOpenedBefore` (and _value _returnvalue)))

(fn `GetSaveName`
  (returns (Name :type String))
  (return (`self.SaveName`)))

(fn `InputCondition`
  (returns (`true can input` :type Boolean))
  (return (not (`self.bOpen`))))

(fn `InputGetToolTipText`
  (returns (Title :type String) (Text :type String))
  (return "按E" "打开（开门钥匙 * 1）"))

(fn `UserConstructionScript`
  (set `/Game/Envoronments/Componments/Inputable.Collision` (`self.Box`) (`self.Inputable`))
  (if (not (> (`KismetStringLibrary.Len` (`self.SaveName`)) 0))
    (set `self.SaveName` (`KismetGuidLibrary.Conv_GuidToString` (`KismetGuidLibrary.NewGuid`)))))