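; Treasure chest prop for multistory dungeons that can open and restore its open state from saved data.
; The construction script fills an empty SaveName with a new GUID, which keys the chest in the world memory GameSaver's bool map.
; IsOpen rotates the lid open if that flag is true.
; Opening plays a timeline and waits briefly, but does not write the flag itself.
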(event `IsOpen`
  (bind _worldmemory (`/Game/JW/WorldMemory/WorldMemoryLibrary.GetWorldMemory`))
  (bind (_value _returnvalue) (`BlueprintMapLibrary.Map_Find` (`/Game/JW/WorldMemory/GameSave/JWSaveGame.BoolMap` (`/Game/JW/WorldMemory/WorldMemory.GameSaver` _worldmemory)) (`self.SaveName`)))
  (if (and _value _returnvalue)
    (`SceneComponent.K2_AddLocalRotation` (`self.Treasure_Chest_lid_01`) (struct :`Roll` -90.0) false false)))

(event `Opening`
  (`TimelineComponent.Play` (`self.Timeline_0`))
  (`KismetSystemLibrary.Delay` 2.0))

(fn `GetSaveName`)

(fn `UserConstructionScript`
  (if (not (> (`KismetStringLibrary.Len` (`self.SaveName`)) 0))
    (set `self.SaveName` (`KismetGuidLibrary.Conv_GuidToString` (`KismetGuidLibrary.NewGuid`)))))